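; Base gun Blueprint that fires hitscan shots from the owning hero's camera and damages EnemyBase_BP targets.
; On BeginPlay, UpdateOwner caches the player pawn as hero and trace-ignored actor.
; Fire checks clip ammo without decrementing it, line-traces, then scales damage by distance, with debug prints.
; The falloff lerp rises toward max damage with distance, minimum damage past dropoff requires negative MaxDamageRange, and Reload is empty.
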(event EventBeginPlay
  (CallFunction|UpdateOwner))

(event EventActorBeginOverlap
  (params (OtherActor :type Actor%20Object%20Reference)))

(event EventTick
  (params (DeltaSeconds :type Float%20%28single-precision%29)))

(fn ConstructionScript)

(fn Fire
  (bind _maxdamage (Variables|Default|GetMaxDamage))
  (bind _mindamage (Variables|Default|GetMinDamage))
  (bind _damagedropoffstart (Variables|Default|GetDamageDropoffStart))
  (bind _mindamage_2 (Variables|Default|GetMinDamage))
  (bind _ownerhero (Variables|Default|GetOwnerHero))
  (bind _camera (Variables|/Game/Blueprints/BaseClasses/HeroBase_BP.HeroBase_BP_C|GetCamera _ownerhero))
  (bind _returnvalue (Transformation|GetWorldLocation _camera))
  (if (> (Variables|Default|GetAmmoInClip) 0)
    (bind _outhit (Collision|LineTraceByChannel _returnvalue (+ _returnvalue (* (Math|Vector|GetForwardVector _camera) (Variables|Default|GetMaxDamageRange))) "TraceTypeQuery1" false (Variables|Default|GetStuffToIgnore) "ForDuration"))
    (Development|PrintString (Utilities|GetDisplayName (.hitactor _outhit)))
    (bind _asenemy_base_bp (Utilities|Casting|CastToEnemyBase_BP (.hitactor _outhit)))
    (if (< (Transformation|GetDistanceTo (Variables|Default|GetOwnerHero) _asenemy_base_bp) (Variables|Default|GetDamageDropoffStart))
      (Default|Damage _asenemy_base_bp _maxdamage)
      (Development|PrintString (Utilities|String|ToString(Float) _maxdamage))
      (elif (> (Transformation|GetDistanceTo (Variables|Default|GetOwnerHero) _asenemy_base_bp) (Variables|Default|GetDamageDropoffStop))
        (if (< (Variables|Default|GetMaxDamageRange) 0.0)
          (Default|Damage _asenemy_base_bp _mindamage)
          (Development|PrintString (Utilities|String|ToString(Float) _mindamage)))
        (else
          (Default|Damage _asenemy_base_bp (+ (* (/ (- (Transformation|GetDistanceTo (Variables|Default|GetOwnerHero) _asenemy_base_bp) _damagedropoffstart) (- (Variables|Default|GetDamageDropoffStop) _damagedropoffstart)) (- (Variables|Default|GetMaxDamage) _mindamage_2)) _mindamage_2))
          (Development|PrintString (Utilities|String|ToString(Float) (+ (* (/ (- (Transformation|GetDistanceTo (Variables|Default|GetOwnerHero) _asenemy_base_bp) _damagedropoffstart) (- (Variables|Default|GetDamageDropoffStop) _damagedropoffstart)) (- (Variables|Default|GetMaxDamage) _mindamage_2)) _mindamage_2))))))))

(fn Reload)

(fn UpdateOwner
  (bind _playerpawnindex (Variables|Default|GetPlayerPawnIndex))
  (bind _stufftoignore (Variables|Default|GetStuffToIgnore))
  (bind _returnvalue (Game|Player|GetPlayerPawn _playerpawnindex))
  (Utilities|Array|Clear _stufftoignore)
  (Utilities|Array|Add _stufftoignore _returnvalue)
  (bind _ashero_base_bp (Utilities|Casting|CastToHeroBase_BP _returnvalue))
  (Variables|Default|SetOwnerHero _ashero_base_bp))